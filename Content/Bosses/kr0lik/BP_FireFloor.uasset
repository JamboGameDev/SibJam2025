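; Timed fire floor hazard for the kr0lik boss that glows, briefly damages Characters that begin overlapping it, then destroys itself.
; The Glow timeline starts on spawn, animating Alpha on a dynamic material created for the plane in the construction script.
; Its event tracks open and close the damage window by toggling actor collision and glow Intensity, calling OnFloorFired when the window closes.
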(event `self.ReceiveBeginPlay`
  (bind (_direction _alpha) (`Timeline|Glow`)
    (:`Update`
      (`MaterialInstanceDynamic.SetScalarParameterValue` (`self.DynamicMatInstance`) "Alpha" _alpha))
    (:`Finished`
      (`self.K2_DestroyActor`))
    (:`DamageTime`
      (`self.SetActorEnableCollision` true)
      (`MaterialInstanceDynamic.SetScalarParameterValue` (`self.DynamicMatInstance`) "Intensity" 10.0))
    (:`DamageDone`
      (`self.SetActorEnableCollision` false)
      (`MaterialInstanceDynamic.SetScalarParameterValue` (`self.DynamicMatInstance`) "Intensity" 5.0)
      (`self.OnFloorFired`))))

(event `self.ReceiveActorBeginOverlap`
  (params (OtherActor :type "Actor Object Reference"))
  (bind _ascharacter (cast `Character` OtherActor))
  (`GameplayStatics.ApplyDamage` _ascharacter (`self.Damage`) null self))

(fn `UserConstructionScript`
  (`self.SetActorEnableCollision` false)
  (bind _returnvalue (`KismetMaterialLibrary.CreateDynamicMaterialInstance` "/Game/Bosses/kr0lik/M_GlowFireFloor.M_GlowFireFloor"))
  (bind _output_get (set `self.DynamicMatInstance` _returnvalue))
  (`PrimitiveComponent.SetMaterial` (`self.Plane`) 0 _output_get))