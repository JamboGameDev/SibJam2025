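; BP_WalkLaser is a laser hazard actor, filed under the kr0lik boss, that travels in a straight line and damages the player character class.
; On BeginPlay, MoveComponentTo slides its Scene component toward a point 10000 units along the actor's forward vector, with Speed serving as the travel duration, then destroys the actor.
; Overlapping a BP_Character applies Damage to it without destroying the laser.
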(event `self.ReceiveBeginPlay`
  (`KismetSystemLibrary.MoveComponentTo` (`self.Scene`) (+ (* (`self.GetActorForwardVector`) 10000.0) (`self.K2_GetActorLocation`)) (`self.K2_GetActorRotation`) false false (`self.Speed`))
  (`self.K2_DestroyActor`))

(event `self.ReceiveActorBeginOverlap`
  (params (OtherActor :type "Actor Object Reference"))
  (bind _asbp_character (cast `/Game/BaseBP/BP_Character` OtherActor))
  (`GameplayStatics.ApplyDamage` _asbp_character (`self.Damage`) null self))

(fn `UserConstructionScript`)