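; BP_Kr0lik is the Blueprint for the Kr0lik boss, adding health-based phase changes on top of its parent class.
; It initializes the phase on BeginPlay after the parent logic runs.
; After parent damage handling, it checks HP against two thresholds, each gated by its own DoOnce so NextPhase fires only once per threshold band.
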(event `self.ReceiveBeginPlay`
  (`parent.ReceiveBeginPlay`)
  (`self.InitPhase`))

(event `self.ReceiveAnyDamage`
  (params (Damage :type "Float (single-precision)") (DamageType :type "DamageType Object Reference") (InstigatedBy :type "Controller Object Reference") (DamageCauser :type "Actor Object Reference"))
  (`parent.ReceiveAnyDamage` Damage DamageType InstigatedBy DamageCauser)
  (if (and (<= (`self.HP`) 7.0) (> (`self.HP`) 3.0))
    (`/Engine/EditorBlueprintResources/StandardMacros.DoOnce` false
      (:`Completed`
        (`self.NextPhase`)))
    (elif (<= (`self.HP`) 3.0)
      (`/Engine/EditorBlueprintResources/StandardMacros.DoOnce` false
        (:`Completed`
          (`self.NextPhase`))))))

(fn `UserConstructionScript`
  (`parent.UserConstructionScript`))