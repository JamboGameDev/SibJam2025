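; Boss attack component for kr0lik that makes the boss leap between waypoints in random order, visiting each once per cycle.
; Each jump launches the character along a high projectile arc computed with a suggested velocity and overridden gravity.
; Tick uses the falling state and a DoOnce to detect landings, then jumps again or, after the last waypoint, triggers the next attack.
; A boss phase change deactivates the attack.
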(event `self.StartAttack`
  (set `self.ActiveAttack` true)
  (`parent.StartAttack`)
  (bind _asbp_boss_base (cast `/Game/Bosses/BP_BossBase` (`self.GetOwner`)))
  (add `/Game/Bosses/BP_BossBase.OnPhaseChange` _asbp_boss_base (delegate `Stop`)))

(event `Stop`
  (if (`self.ActiveAttack`)
    (set `self.ActiveAttack` false)))

(event `self.ReceiveTick`
  (params (DeltaSeconds :type "Float (single-precision)"))
  (if (`self.ActiveAttack`)
    (bind _asbp_boss_base (cast `/Game/Bosses/BP_BossBase` (`self.GetOwner`)))
    (if (`NavMovementComponent.IsFalling` (`Character.CharacterMovement` _asbp_boss_base))
      (goto _label :!via `Reset`)
      (else
        (`/Engine/EditorBlueprintResources/StandardMacros.DoOnce` true :!label _label
          (:`Completed`
            (`self.MoveFinished` null)
            (if (== (`self.CurrentWaypoint`) 0)
              (`KismetSystemLibrary.Delay` (`self.AttacksDelay`))
              (`self.AllMovesFinished`)
              (set `self.ActiveAttack` false)
              (`self.CallBossNextAttack`)
              (else
                (`KismetSystemLibrary.Delay` 1.5)
                (if (`self.ActiveAttack`)
                  (`self.MoveToWaypoint`))))))))))

(event `self.MoveToWaypoint`
  (bind _asbp_boss_base (cast `/Game/Bosses/BP_BossBase` (`self.GetOwner`)))
  (`|ExecutionSequence`
    (:`then_0`
      (set `self.SelectedWaypoint` null)
      (while (not (`KismetSystemLibrary.IsValid` (`self.SelectedWaypoint`)))
        (bind _output_get (set `self.SelectedWaypoint` (`KismetArrayLibrary.Array_Random` (`self.Waypoints`))))
        (if (`KismetArrayLibrary.Array_Contains` (`self.PreviousWaypoints`) _output_get)
          (set `self.SelectedWaypoint` null)
          (else
            (`KismetArrayLibrary.Array_Add` (`self.PreviousWaypoints`) (`self.SelectedWaypoint`))))))
    (:`then_1`
      (`self.MoveStarted`)
      (bind _tossvelocity (`GameplayStatics.BlueprintSuggestProjectileVelocity` (`Actor.K2_GetActorLocation` _asbp_boss_base) (+ (`Actor.K2_GetActorLocation` (`self.SelectedWaypoint`)) (0.0 0.0 10.0)) 2000.0 -2940.0 "DoNotTrace" 0.0 true))
      (`Character.LaunchCharacter` _asbp_boss_base _tossvelocity true true)
      (`/Engine/EditorBlueprintResources/StandardMacros.IncrementInt` (`self.CurrentWaypoint`)
        (:`  `
          (if (== (`self.CurrentWaypoint`) (`KismetArrayLibrary.Array_Length` (`self.Waypoints`)))
            (set `self.CurrentWaypoint` 0)
            (`KismetArrayLibrary.Array_Clear` (`self.PreviousWaypoints`))))))))