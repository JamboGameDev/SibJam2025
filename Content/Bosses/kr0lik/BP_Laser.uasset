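; Boss laser projectile in the kr0lik boss folder that sweeps in a straight line and damages any BP_Character it overlaps.
; On BeginPlay it slides its static mesh far along X or Y, chosen by MoveAlongX and signed by MoveTo, then destroys itself when the timed move ends.
; The move target is built from the actor's world location and rotation but passed as the component's relative transform.
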(event `self.ReceiveBeginPlay`
  (bind _returnvalue (`self.K2_GetActorRotation`))
  (bind (__moveto_x __moveto_y) (`KismetMathLibrary.BreakVector` (`self. MoveTo`)))
  (bind _staticmesh (`self.StaticMesh`))
  (if (`self.MoveAlongX`)
    (`KismetSystemLibrary.MoveComponentTo` _staticmesh (+ (`self.K2_GetActorLocation`) (`KismetMathLibrary.MakeVector` (* (`KismetMathLibrary.SignOfFloat` __moveto_x) 10000.0))) _returnvalue false false 7.0)
    (else
      (`KismetSystemLibrary.MoveComponentTo` _staticmesh (+ (`self.K2_GetActorLocation`) (`KismetMathLibrary.MakeVector` 0.0 (* (`KismetMathLibrary.SignOfFloat` __moveto_y) 10000.0))) _returnvalue false false 7.0)))
  (`self.K2_DestroyActor`))

(event `self.ReceiveActorBeginOverlap`
  (params (OtherActor :type "Actor Object Reference"))
  (bind _asbp_character (cast `/Game/BaseBP/BP_Character` OtherActor))
  (`GameplayStatics.ApplyDamage` _asbp_character (`self.Damage`)))

(fn `UserConstructionScript`)