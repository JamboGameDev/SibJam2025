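; Boss attack component that runs a fire-floor attack, raising one random hill out of the ground while the floor is active.
; On BeginPlay it spawns a hill at each HillsPoint, sunk just below that point using its bounds height.
; ExecuteAttack spawns a large BP_FireFloor beneath the owner and ascends the chosen hill.
; The floor's OnFloorFired event lowers that hill, then triggers the boss's next attack after a delay.
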(event `self.ReceiveBeginPlay`
  (for _array_element (`self.HillsPoint`)
    (bind _returnvalue (`|SpawnActorFromClass` "/Game/Bosses/kr0lik/BP_Hill.BP_Hill_C" (`KismetMathLibrary.MakeTransform` (`Actor.K2_GetActorLocation` _array_element) (struct) (4.0 4.0 1.1)) "Undefined" "OverrideRootScale" null null))
    (`Actor.K2_SetActorLocation` _returnvalue (- (`Actor.K2_GetActorLocation` _returnvalue) (`KismetMathLibrary.MakeVector` 0.0 0.0 (.z (`.BoxExtent` (`Actor.GetActorBounds` _returnvalue false false)))) (0.0 0.0 10.0)) false false)
    (`KismetArrayLibrary.Array_Add` (`self.Hills`) _returnvalue)))

(event `self.ExecuteAttack`
  (bind _returnvalue (`|SpawnActorFromClass` "/Game/Bosses/kr0lik/BP_FireFloor.BP_FireFloor_C" (`KismetMathLibrary.MakeTransform` (- (`Actor.K2_GetActorLocation` (`self.GetOwner`)) (0.0 0.0 50.0)) (struct) (30.0 30.0 1.0)) "AlwaysSpawn" "OverrideRootScale" null null))
  (add `/Game/Bosses/kr0lik/BP_FireFloor.OnFloorFired` _returnvalue (delegate `FinishAttack`))
  (bind _output_get (set `self.AscendedHill` (`KismetArrayLibrary.Array_Random` (`self.Hills`))))
  (`/Game/Bosses/kr0lik/BP_Hill.Ascend` _output_get))

(event `FinishAttack`
  (`/Game/Bosses/kr0lik/BP_Hill.Descend` (`self.AscendedHill`))
  (`KismetSystemLibrary.Delay` (`self.AttacksDelay`))
  (`self.CallBossNextAttack`))