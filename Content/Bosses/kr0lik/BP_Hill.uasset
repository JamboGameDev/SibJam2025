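; BP_Hill is a hill actor in the kr0lik boss folder that can rise and sink through its Ascend and Descend events.
; Each event moves the StaticMesh over one second to the actor's bounds origin, offset up or down by its full bounding height.
; Bounds are read at call time, and their world-space origin feeds directly into the mesh's relative-location target.
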(event `Ascend`
  (bind (_origin _boxextent) (`self.GetActorBounds` false))
  (`KismetSystemLibrary.MoveComponentTo` (`self.StaticMesh`) (+ _origin (* (`KismetMathLibrary.MakeVector` 0.0 0.0 (.z _boxextent)) 2)) (struct) false false 1.0))

(event `Descend`
  (bind (_origin _boxextent) (`self.GetActorBounds` false))
  (`KismetSystemLibrary.MoveComponentTo` (`self.StaticMesh`) (- _origin (* (`KismetMathLibrary.MakeVector` 0.0 0.0 (.z _boxextent)) 2)) (struct) false false 1.0))

(fn `UserConstructionScript`)