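; Boss attack component for kr0lik that leaps at the player and fires a ring of shells on landing.
; ExecuteAttack launches the owning boss along a high arc computed with SuggestProjectileVelocity toward the player's position.
; Tick, active only during the attack, watches the movement's falling state through a DoOnce to detect touchdown.
; Landing spawns outward-facing BP_BossShell actors evenly around the boss, then triggers the next attack after a delay.
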(event `self.StartAttack`
  (`self.SetComponentTickEnabled` true)
  (`parent.StartAttack`))

(event `self.ReceiveTick`
  (params (DeltaSeconds :type "Float (single-precision)"))
  (bind _asbp_boss_base (cast `/Game/Bosses/BP_BossBase` (`self.GetOwner`)))
  (if (`NavMovementComponent.IsFalling` (`Character.CharacterMovement` _asbp_boss_base))
    (goto _label :!via `Reset`)
    (else
      (`/Engine/EditorBlueprintResources/StandardMacros.DoOnce` true :!label _label
        (:`Completed`
          (`self.SetComponentTickEnabled` false)
          (`self.Landed`))))))

(event `self.ExecuteAttack`
  (bind _returnvalue (`self.GetOwner`))
  (bind _tossvelocity (`GameplayStatics.BlueprintSuggestProjectileVelocity` (`Actor.K2_GetActorLocation` _returnvalue) (`Actor.K2_GetActorLocation` (`GameplayStatics.GetPlayerCharacter` 0)) 1750.0 0.0 "DoNotTrace" 0.0 true))
  (bind _asbp_boss_base (cast `/Game/Bosses/BP_BossBase` _returnvalue))
  (`Character.LaunchCharacter` _asbp_boss_base _tossvelocity true true))

(event `Landed`
  (for _index (range 360)
    (if (not (!= (mod _index 6) 0))
      (bind _returnvalue (`KismetMathLibrary.MakeRotator` 0.0 0.0 (`KismetMathLibrary.Conv_IntToDouble` _index)))
      (`|SpawnActorFromClass` "/Game/Bosses/Babka/BP_BossShell.BP_BossShell_C" (`KismetMathLibrary.MakeTransform` (+ (`Actor.K2_GetActorLocation` (`self.GetOwner`)) (* (`KismetMathLibrary.GetForwardVector` _returnvalue) 200)) _returnvalue) "Undefined" "OverrideRootScale" null null)))
  (`KismetSystemLibrary.Delay` (`self.AttacksDelay`))
  (`self.CallBossNextAttack`))