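; Boss attack component for kr0lik that leaps the boss to a waypoint and fires lasers.
; MovetoWaypoint launches the owning BP_BossBase along a high-arc suggested projectile velocity to a random waypoint, or attacks immediately if none exist.
; While active, Tick watches falling state through a DoOnce to attack once per landing.
; ExecuteAttack spawns two perpendicular BP_Laser actors using the waypoint's forward vector, then calls the next boss attack after a delay.
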(event `self.StartAttack`
  (set `self.ActiveAttack` true)
  (`parent.StartAttack`))

(event `self.ReceiveTick`
  (params (DeltaSeconds :type "Float (single-precision)"))
  (if (`self.ActiveAttack`)
    (bind _asbp_boss_base (cast `/Game/Bosses/BP_BossBase` (`self.GetOwner`)))
    (if (`KismetSystemLibrary.IsValid` (`self.PickedWaypoint`))
      (if (`NavMovementComponent.IsFalling` (`Character.CharacterMovement` _asbp_boss_base))
        (goto _label :!via `Reset`)
        (else
          (`/Engine/EditorBlueprintResources/StandardMacros.DoOnce` true :!label _label
            (:`Completed`
              (`self.ExecuteAttack`))))))))

(event `self.MoveToWaypoint`
  (bind _asbp_boss_base (cast `/Game/Bosses/BP_BossBase` (`self.GetOwner`)))
  (if (`KismetArrayLibrary.Array_IsEmpty` (`self.Waypoints`))
    (`self.ExecuteAttack`)
    (else
      (bind _output_get (set `self.PickedWaypoint` (`KismetArrayLibrary.Array_Random` (`self.Waypoints`))))
      (`self.MoveStarted`)
      (bind _tossvelocity (`GameplayStatics.BlueprintSuggestProjectileVelocity` (`Actor.K2_GetActorLocation` _asbp_boss_base) (+ (`Actor.K2_GetActorLocation` _output_get) (0.0 0.0 10.0)) 1750.0 0.0 "DoNotTrace" 0.0 true))
      (`Character.LaunchCharacter` _asbp_boss_base _tossvelocity true true)
      (`/Engine/EditorBlueprintResources/StandardMacros.IncrementInt` (`self.CurrentWaypoint`)
        (:`  `
          (if (== (`self.CurrentWaypoint`) (`KismetArrayLibrary.Array_Length` (`self.Waypoints`)))
            (set `self.CurrentWaypoint` 0)))))))

(event `self.ExecuteAttack`
  (`|SpawnActorFromClass` "/Game/Bosses/kr0lik/BP_Laser.BP_Laser_C" (`KismetMathLibrary.MakeTransform` (`Actor.K2_GetActorLocation` (`self.GetOwner`)) (struct :`Yaw` 90.0 :`Roll` 90.0) (0.25 0.25 50.0)) "Undefined" "OverrideRootScale" null false (`SceneComponent.GetForwardVector` (`/Game/Bosses/Attacks/BP_BossWaypoint.DefaultSceneRoot` (`self.PickedWaypoint`))) null)
  (`|SpawnActorFromClass` "/Game/Bosses/kr0lik/BP_Laser.BP_Laser_C" (`KismetMathLibrary.MakeTransform` (`Actor.K2_GetActorLocation` (`self.GetOwner`)) (struct :`Roll` 90.0) (0.25 0.25 50.0)) "Undefined" "OverrideRootScale" null true (`SceneComponent.GetForwardVector` (`/Game/Bosses/Attacks/BP_BossWaypoint.DefaultSceneRoot` (`self.PickedWaypoint`))) null)
  (`KismetSystemLibrary.Delay` (`self.AttacksDelay`))
  (set `self.ActiveAttack` false)
  (`self.CallBossNextAttack`))