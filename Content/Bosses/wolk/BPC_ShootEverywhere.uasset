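; Boss attack component that sprays BP_BossShell actors from randomly picked shooting points for a set duration.
; StartAttack clears the stop flag and starts ExecuteAttack, which spawns a shell and calls itself again after a short random delay.
; A DoOnce-gated timer fires StopAttack after AttackDuration, so the loop exits and, after AttacksDelay, calls the boss's next attack.
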(event `self.StartAttack`
  (set `self.ShouldStopAttack` false)
  (`self.ExecuteAttack`)
  (goto _label :!via `Reset`))

(event `self.ExecuteAttack`
  (bind _outitem (`KismetArrayLibrary.Array_Random` (`self.ShootingPoints`)))
  (if (`self.ShouldStopAttack`)
    (`KismetSystemLibrary.Delay` (`self.AttacksDelay`))
    (`self.CallBossNextAttack`)
    (else
      (`|ExecutionSequence`
        (:`then_0`
          (`/Engine/EditorBlueprintResources/StandardMacros.DoOnce` false :!label _label
            (:`Completed`
              (`KismetSystemLibrary.K2_SetTimerDelegate` (delegate `StopAttack`) (`self.AttackDuration`)))))
        (:`then_1`
          (`|SpawnActorFromClass` "/Game/Bosses/Babka/BP_BossShell.BP_BossShell_C" (`KismetMathLibrary.MakeTransform` (`Actor.K2_GetActorLocation` _outitem) (`Actor.K2_GetActorRotation` _outitem)) "Undefined" "OverrideRootScale" null null)
          (`KismetSystemLibrary.Delay` (`KismetMathLibrary.RandomFloatInRange` 0.2 0.5))
          (`self.ExecuteAttack`))))))

(event `StopAttack`
  (set `self.ShouldStopAttack` true))