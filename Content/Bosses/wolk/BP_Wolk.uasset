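; BP_Wolk is a timed boss that ends when its countdown expires, built on a parent boss Blueprint.
; On activation it sets one-shot timers at fractions of StartTime to advance phases twice, then a final one that destroys the actor, plays end dialogue and calls Drop.
; It creates a boss timer widget fed by StartTime as its boss UI.
; Its AnyDamage event is empty, with no parent call.
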(event `self.ReceiveBeginPlay`
  (`parent.ReceiveBeginPlay`))

(event `self.ActivateBoss`
  (`parent.ActivateBoss`)
  (`KismetSystemLibrary.K2_SetTimerDelegate` (delegate `TimeIsUp`) (`self.StartTime`))
  (`KismetSystemLibrary.K2_SetTimerDelegate` (delegate `Phase2`) (* (`self.StartTime`) 0.3))
  (`KismetSystemLibrary.K2_SetTimerDelegate` (delegate `Phase3`) (* (`self.StartTime`) 0.7)))

(event `TimeIsUp`
  (`self.K2_DestroyActor`)
  (`self.PlayEndDialogue`)
  (`self.Drop`))

(event `Phase3`
  (`self.NextPhase`))

(event `Phase2`
  (`self.NextPhase`))

(event `self.CreateBossWidget`
  (bind _returnvalue (`|CreateWidget` "/Game/Bosses/WBP_BossTimer.WBP_BossTimer_C" null (`self.StartTime`)))
  (`UserWidget.AddToViewport` _returnvalue 0)
  (set `self.BossWidget` _returnvalue))

(event `self.ReceiveAnyDamage`
  (params (Damage :type "Float (single-precision)") (DamageType :type "DamageType Object Reference") (InstigatedBy :type "Controller Object Reference") (DamageCauser :type "Actor Object Reference")))

(fn `UserConstructionScript`
  (`parent.UserConstructionScript`))