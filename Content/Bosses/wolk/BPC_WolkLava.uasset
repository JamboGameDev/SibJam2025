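; BPC_WolkLava is an attack component for the Wolk boss that spawns bolts of light at lava points.
; StartAttack copies the lava points into a working list, then runs the parent start.
; ExecuteAttack spawns an enlarged BP_BoltOfLight just above a random point, removes that point, and calls itself after a short delay.
; Once the list is empty, it waits AttacksDelay and triggers the boss's next attack.
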(event `self.StartAttack`
  (set `self.UsedLavaPoints` (`self.LavaPoints`))
  (`parent.StartAttack`))

(event `self.ExecuteAttack`
  (bind _usedlavapoints (`self.UsedLavaPoints`))
  (if (`KismetArrayLibrary.Array_IsEmpty` _usedlavapoints)
    (`KismetSystemLibrary.Delay` (`self.AttacksDelay`))
    (`self.CallBossNextAttack`)
    (else
      (bind _output_get (set `self.TmpLavaPoint` (`KismetArrayLibrary.Array_Random` _usedlavapoints)))
      (`|SpawnActorFromClass` "/Game/Bosses/Babka/BP_BoltOfLight.BP_BoltOfLight_C" (`KismetMathLibrary.MakeTransform` (+ (`Actor.K2_GetActorLocation` _output_get) (0.0 0.0 20.0)) (struct) (5.0 5.0 5.0)) "Undefined" "OverrideRootScale" null null)
      (`KismetArrayLibrary.Array_RemoveItem` (`self.UsedLavaPoints`) (`self.TmpLavaPoint`))
      (`KismetSystemLibrary.Delay` 0.1)
      (`self.ExecuteAttack`))))