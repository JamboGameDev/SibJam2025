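; Base boss attack component for BP_BossBase, with an empty ExecuteAttack event as the attack hook.
; StartAttack calls ExecuteAttack directly without waypoints; otherwise it moves the boss to the current waypoint via AIMoveTo.
; Success and failure alike advance the looping index and signal move finished, plus all moves finished on wrap.
; CallBossNextAttack hands control back by calling the boss's StartAttack.
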(event `StartAttack`
  (`self.MoveToWaypoint`))

(event `MoveToWaypoint`
  (bind _asbp_boss_base (cast `/Game/Bosses/BP_BossBase` (`self.GetOwner`)))
  (if (`KismetArrayLibrary.Array_IsEmpty` (`self.Waypoints`))
    (`self.ExecuteAttack`)
    (else
      (`self.MoveStarted`)
      (`|AIMoveTo` _asbp_boss_base (0.0 0.0 0.0) (`|GetArrayItem` (`self.Waypoints`) (`self.CurrentWaypoint`))
        (:`OnSuccess`
          _)
        (:`OnFail`
          _))
      (`/Engine/EditorBlueprintResources/StandardMacros.IncrementInt` (`self.CurrentWaypoint`)
        (:`  `
          (if (== (`self.CurrentWaypoint`) (`KismetArrayLibrary.Array_Length` (`self.Waypoints`)))
            (set `self.CurrentWaypoint` 0)
            (`self.AllMovesFinished`))
          (`self.MoveFinished`))))))

(event `ExecuteAttack`)

(fn `CallBossNextAttack`
  (bind _asbp_boss_base (cast `/Game/Bosses/BP_BossBase` (`self.GetOwner`)))
  (`/Game/Bosses/BP_BossBase.StartAttack` _asbp_boss_base))