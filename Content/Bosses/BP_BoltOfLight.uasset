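; BP_BoltOfLight is a boss attack actor that shows a warning plane, then turns it into an invisible damage area.
; Construction shows the plane without collision, and after a short delay on BeginPlay it hides and becomes query-only.
; A BP_Character that begins overlapping the plane takes Damage, and the actor destroys itself when its Niagara system finishes.
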(event `self.ReceiveBeginPlay`
  (bind _plane (`self.Plane`))
  (`KismetSystemLibrary.Delay` 0.8)
  (`PrimitiveComponent.SetCollisionEnabled` _plane "QueryOnly")
  (`SceneComponent.SetHiddenInGame` _plane true false))

(event `self.Plane.OnComponentBeginOverlap`
  (params (OverlappedComponent :type "PrimitiveComponent Object Reference") (OtherActor :type "Actor Object Reference") (OtherComp :type "PrimitiveComponent Object Reference") (OtherBodyIndex :type Integer) (bFromSweep :type Boolean) (SweepResult :type "HitResult Structure (by ref)"))
  (bind _asbp_character (cast `/Game/BaseBP/BP_Character` OtherActor))
  (`GameplayStatics.ApplyDamage` _asbp_character (`self.Damage`)))

(event `self.Niagara.OnSystemFinished`
  (params (PSystem :type "NiagaraComponent Object Reference"))
  (`self.K2_DestroyActor`))

(fn `UserConstructionScript`
  (bind _plane (`self.Plane`))
  (`PrimitiveComponent.SetCollisionEnabled` _plane "NoCollision")
  (`SceneComponent.SetHiddenInGame` _plane false false))