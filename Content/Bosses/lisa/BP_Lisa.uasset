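; BP_Lisa is the Blueprint for the Lisa boss, which spawns minions and advances through phases as its health drops.
; On BeginPlay it runs parent setup, initializes the phase and starts a self-calling event that spawns a minion at the Spawner component every second, with no stop condition.
; After parent damage handling, two HP thresholds each trigger NextPhase through their own DoOnce.
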(event `self.ReceiveBeginPlay`
  (`parent.ReceiveBeginPlay`)
  (`self.InitPhase`)
  (`self.SpawnMinions`))

(event `SpawnMinions`
  (`|SpawnActorFromClass` (`self.MinionClass`) (`KismetMathLibrary.MakeTransform` (`SceneComponent.K2_GetComponentLocation` (`self.Spawner`))) "Undefined" "OverrideRootScale" null null)
  (`KismetSystemLibrary.Delay` 1.0)
  (`self.SpawnMinions`))

(event `self.ReceiveAnyDamage`
  (params (Damage :type "Float (single-precision)") (DamageType :type "DamageType Object Reference") (InstigatedBy :type "Controller Object Reference") (DamageCauser :type "Actor Object Reference"))
  (`parent.ReceiveAnyDamage` Damage DamageType InstigatedBy DamageCauser)
  (if (and (<= (`self.HP`) 7.0) (> (`self.HP`) 3.0))
    (`/Engine/EditorBlueprintResources/StandardMacros.DoOnce` false
      (:`Completed`
        (`self.NextPhase`)))
    (elif (<= (`self.HP`) 3.0)
      (`/Engine/EditorBlueprintResources/StandardMacros.DoOnce` false
        (:`Completed`
          (`self.NextPhase`))))))

(fn `UserConstructionScript`
  (`parent.UserConstructionScript`))