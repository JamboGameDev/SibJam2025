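; BPC_LisaLasers is an attack component for the Lisa boss that lays down walking lasers along a waypoint path.
; On BeginPlay it binds to the move-finished and all-moves-finished events.
; Each finished move spawns a BP_WalkLaser at that waypoint's location and rotation, with configurable length and speed, then starts the next move.
; When all moves finish, it waits AttacksDelay and calls the boss's next attack.
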(event `self.ReceiveBeginPlay`
  (add `self.MoveFinished` (delegate `SpawnLaser`))
  (add `self.AllMovesFinished` (delegate `NextAttack`)))

(event `NextAttack`
  (`KismetSystemLibrary.Delay` (`self.AttacksDelay`))
  (`self.CallBossNextAttack`))

(event `SpawnLaser` :!signature `self.MoveFinished`
  (params (WaypointDone :type "/Game/Bosses/Attacks/BP_BossWaypoint Object Reference"))
  (`|SpawnActorFromClass` "/Game/Bosses/kr0lik/BP_WalkLaser.BP_WalkLaser_C" (`KismetMathLibrary.MakeTransform` (`Actor.K2_GetActorLocation` WaypointDone) (`Actor.K2_GetActorRotation` WaypointDone) (`KismetMathLibrary.MakeVector` 1.0 1.0 (`self.LaserLength`))) "Undefined" "OverrideRootScale" null (`self.LaserSpeed`) null)
  (`self.MoveToWaypoint`))