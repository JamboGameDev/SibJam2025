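; BPC_Trail is a boss attack component for Lisa that leaves a trail of enlarged BP_BoltOfLight actors as the boss moves.
; StartAttack runs the parent attack and arms a one-shot timer that spawns a bolt at the owner's transform every Frequency, re-arming while IsAtackActive is true.
; Move-finished events trigger the next waypoint move.
; Finishing all moves, or a timer tick finding the attack inactive, calls the boss's next attack.
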(event `self.StartAttack`
  (set `self.IsAtackActive` true)
  (`parent.StartAttack`)
  (`KismetSystemLibrary.K2_SetTimerDelegate` (delegate `self.ExecuteAttack`) (`self.Frequency`)))

(event `self.ReceiveBeginPlay`
  (add `self.AllMovesFinished` (delegate `AttackDone`))
  (add `self.MoveFinished` (delegate `OnMoveFinished`)))

(event `OnMoveFinished` :!signature `self.MoveFinished`
  (params (WaypointDone :type "/Game/Bosses/Attacks/BP_BossWaypoint Object Reference"))
  (`self.MoveToWaypoint`))

(event `AttackDone`
  (`self.CallBossNextAttack`))

(event `self.ExecuteAttack`
  (bind _returnvalue (`self.GetOwner`))
  (`|SpawnActorFromClass` "/Game/Bosses/Babka/BP_BoltOfLight.BP_BoltOfLight_C" (`KismetMathLibrary.MakeTransform` (`Actor.K2_GetActorLocation` _returnvalue) (`Actor.K2_GetActorRotation` _returnvalue) (5.0 5.0 5.0)) "Undefined" "OverrideRootScale" null null)
  (if (`self.IsAtackActive`)
    (`KismetSystemLibrary.K2_SetTimerDelegate` (delegate `self.ExecuteAttack`) (`self.Frequency`))
    (else
      (`self.CallBossNextAttack`))))