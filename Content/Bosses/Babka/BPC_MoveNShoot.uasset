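; Boss attack component for Babka that fires repeatedly while the boss moves between waypoints.
; Move-finished events chain to the next waypoint, and the first move start launches a do-once, self-recalling spawn loop paced by FireRate.
; When all moves finish, the loop waits AttacksDelay, calls the boss's next attack and resets.
; Spawn location comes from the owner's forward vector plus an X offset, without the owner's position.
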(event `InitAttack`
  (`/Engine/EditorBlueprintResources/StandardMacros.DoOnce` false :!label _label
    (:`Completed`
      (`KismetSystemLibrary.Delay` (`self.FireRate`))
      (`self.ExecuteAttack`))))

(event `self.ExecuteAttack`
  (bind (_returnvalue_x _returnvalue_y _returnvalue_z) (`KismetMathLibrary.BreakVector` (`Actor.GetActorForwardVector` (`self.GetOwner`))))
  (if (`self.IsMoveFinished`)
    (`KismetSystemLibrary.Delay` (`self.AttacksDelay`))
    (`self.CallBossNextAttack`)
    (set `self.IsMoveFinished` false)
    (goto _label :!via `Reset`)
    (else
      (`|SpawnActorFromClass` "/Game/Bosses/Babka/BP_BossShell.BP_BossShell_C" (`KismetMathLibrary.MakeTransform` (`KismetMathLibrary.MakeVector` (+ _returnvalue_x 100.0) _returnvalue_y _returnvalue_z) (struct :`Yaw` 180.0)) "Undefined" "OverrideRootScale" null null)
      (`KismetSystemLibrary.Delay` (`self.FireRate`))
      (`self.ExecuteAttack`))))

(event `self.ReceiveBeginPlay`
  (add `self.AllMovesFinished` (delegate `SetMoveFinished`))
  (add `self.MoveFinished` (delegate `NextMove`))
  (add `self.MoveStarted` (delegate `InitAttack`)))

(event `SetMoveFinished`
  (set `self.IsMoveFinished` true))

(event `NextMove`
  (if (not (`self.IsMoveFinished`))
    (`self.MoveToWaypoint`)))