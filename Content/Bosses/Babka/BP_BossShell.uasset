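; BP_BossShell is a damaging shell actor, filed under the Babka boss, that hurts the player character on overlap.
; It applies its Damage value to BP_Character and then destroys itself, or expires five seconds after spawning.
; A chain of casts lets it ignore other shells, lasers, light bolts, bullets and checkpoints, while overlapping any other actor destroys it.
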(event `self.ReceiveBeginPlay`
  (`KismetSystemLibrary.Delay` 5.0)
  (`self.K2_DestroyActor`))

(event `self.ReceiveActorBeginOverlap`
  (params (OtherActor :type "Actor Object Reference"))
  (bind _asbp_character (cast `/Game/BaseBP/BP_Character` OtherActor)
    (:`then`
      (`GameplayStatics.ApplyDamage` _asbp_character (`self.Damage`) null self))
    (:`CastFailed`
      (cast `/Game/Bosses/Babka/BP_BossShell` OtherActor
        (:`CastFailed`
          (cast `/Game/Bosses/kr0lik/BP_Laser` OtherActor
            (:`CastFailed`
              (cast `/Game/Bosses/kr0lik/BP_WalkLaser` OtherActor
                (:`CastFailed`
                  (cast `/Game/Bosses/Babka/BP_BoltOfLight` OtherActor
                    (:`CastFailed`
                      (cast `/Game/CAP_DIMA/BP/Blueprints/Bullet` OtherActor
                        (:`CastFailed`
                          (cast `/Game/CAP_DIMA/BP/Blueprints/Checpoint` OtherActor
                            (:`CastFailed`
                              _))))))))))))))
  (`self.K2_DestroyActor`))

(fn `UserConstructionScript`)