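; Boss attack component for Babka that drops a scaled-up BP_BoltOfLight at each stop along a waypoint path.
; On BeginPlay it binds to the move-finished event, and each completed move spawns a bolt just above the owner's location.
; It keeps moving until the current waypoint index is 0, then waits the attack delay and calls StartAttack on the owning BP_BossBase.
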(event `MoveFinishedEvent` :!signature `self.MoveFinished`
  (params (NewParam :type "/Game/Bosses/Attacks/BP_BossWaypoint Object Reference"))
  (`self.ExecuteAttack`))

(event `self.ExecuteAttack`
  (`|SpawnActorFromClass` "/Game/Bosses/Babka/BP_BoltOfLight.BP_BoltOfLight_C" (`KismetMathLibrary.MakeTransform` (- (`Actor.K2_GetActorLocation` (`self.GetOwner`)) (0.0 0.0 -30.0)) (struct) (5.0 5.0 5.0)) "Undefined" "OverrideRootScale" null null)
  (if (== (`self.CurrentWaypoint`) 0)
    (bind _asbp_boss_base (cast `/Game/Bosses/BP_BossBase` (`self.GetOwner`)))
    (`KismetSystemLibrary.Delay` (`self.AttacksDelay`))
    (`/Game/Bosses/BP_BossBase.StartAttack` _asbp_boss_base)
    (else
      (`self.MoveToWaypoint`))))

(event `self.ReceiveBeginPlay`
  (add `self.MoveFinished` (delegate `MoveFinishedEvent`)))