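; Boss attack component for Babka that fires a randomly spread stream of shells from the owner's position.
; ExecuteAttack resets the elapsed-time counter and starts a chain of one-shot timers with random delays up to FireRate.
; Each SpawnShell spawns a half-scale BP_BossShell, then adds a random yaw to the firing rotator.
; Once accumulated delays exceed FireTime, it calls StartAttack on the owning BP_BossBase instead of rescheduling.
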(event `self.ExecuteAttack`
  (set `self.DeltaFireRate` 0.0)
  (`KismetSystemLibrary.K2_SetTimerDelegate` (delegate `SpawnShell`) (`KismetMathLibrary.RandomFloatInRange` 0.0 (`self.FireRate`))))

(event `SpawnShell`
  (bind (_returnvalue_roll _returnvalue_pitch _returnvalue_yaw) (`KismetMathLibrary.BreakRotator` (`KismetMathLibrary.RandomRotator` false)))
  (`|SpawnActorFromClass` "/Game/Bosses/Babka/BP_BossShell.BP_BossShell_C" (`KismetMathLibrary.MakeTransform` (+ (* (`KismetMathLibrary.GetForwardVector` (`self.Rotator`)) 100.0) (`Actor.K2_GetActorLocation` (`self.GetOwner`))) (`self.Rotator`) (0.5 0.5 0.5)) "Undefined" "OverrideRootScale" null null)
  (set `self.Rotator` (`KismetMathLibrary.ComposeRotators` (`self.Rotator`) (`KismetMathLibrary.MakeRotator` 0.0 0.0 _returnvalue_yaw)))
  (bind _output_get (set `self.NextShotFiresIn` (`KismetMathLibrary.RandomFloatInRange` 0.0 (`self.FireRate`))))
  (set `self.DeltaFireRate` (+ _output_get (`self.DeltaFireRate`)))
  (if (> (`self.DeltaFireRate`) (`self.FireTime`))
    (bind _asbp_boss_base (cast `/Game/Bosses/BP_BossBase` (`self.GetOwner`)))
    (`/Game/Bosses/BP_BossBase.StartAttack` _asbp_boss_base)
    (else
      (`KismetSystemLibrary.K2_SetTimerDelegate` (delegate `SpawnShell`) (`self.NextShotFiresIn`)))))