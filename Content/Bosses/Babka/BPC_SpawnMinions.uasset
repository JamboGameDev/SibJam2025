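; Boss attack component in the Babka boss folder that spawns a batch of minions at its owner's location.
; ExecuteAttack spawns one MinionClass actor with a random sideways Y offset, then re-calls itself after a short delay until NumberOfMinions is reached.
; It then resets the counter, waits PostAttackDelay and calls StartAttack on the owning BP_BossBase to resume the boss's attacks.
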(event `self.ExecuteAttack`
  (bind (_returnvalue_x _returnvalue_y _returnvalue_z) (`KismetMathLibrary.BreakVector` (`Actor.K2_GetActorLocation` (`self.GetOwner`))))
  (`|SpawnActorFromClass` (`self.MinionClass`) (`KismetMathLibrary.MakeTransform` (`KismetMathLibrary.MakeVector` _returnvalue_x (+ _returnvalue_y (* (`KismetMathLibrary.RandomIntegerInRange` -1 1) 100)) _returnvalue_z)) "Undefined" "OverrideRootScale" null null)
  (`KismetSystemLibrary.Delay` 0.5)
  (`/Engine/EditorBlueprintResources/StandardMacros.IncrementInt` (`self.CurrentSpawned`)
    (:`  `
      (if (>= (`self.CurrentSpawned`) (`self.NumberOfMinions`))
        (bind _asbp_boss_base (cast `/Game/Bosses/BP_BossBase` (`self.GetOwner`)))
        (set `self.CurrentSpawned` 0)
        (`KismetSystemLibrary.Delay` (`self.PostAttackDelay`))
        (`/Game/Bosses/BP_BossBase.StartAttack` _asbp_boss_base)
        (else
          (`self.ExecuteAttack`))))))