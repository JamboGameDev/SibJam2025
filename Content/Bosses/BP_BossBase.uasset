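; Base boss actor that activates once, shows an HP widget, takes damage, and on death opens end dialogue, spawns a drop and destroys itself.
; Each phase collects BPC_BossAttack components whose tags match the phase enum name, with every StartAttack call advancing cyclically through them.
; NextPhase increments the enum, fires a phase-change call and rebuilds the attack list; nothing here triggers it.
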(event `self.ReceiveBeginPlay`
  (add `self.OnDestroyed` (delegate `Cleanup`)))

(event `Cleanup` :!signature `self.OnDestroyed`
  (params (DestroyedActor :type "Actor Object Reference"))
  (`Widget.RemoveFromParent` (`self.BossWidget`)))

(event `CreateBossWidget`
  (bind _returnvalue (`|CreateWidget` "/Game/Bosses/WBP_BossHP.WBP_BossHP_C" null self (`self.HP`)))
  (`UserWidget.AddToViewport` _returnvalue 0)
  (set `self.BossWidget` _returnvalue))

(event `InitPhase`
  (`KismetArrayLibrary.Array_Clear` (`self.CurrentAttacks`))
  (for _array_element (`self.K2_GetComponentsByClass` "/Game/Bosses/Attacks/BPC_BossAttack.BPC_BossAttack_C")
    (if (`KismetArrayLibrary.Array_Contains` (`ActorComponent.ComponentTags` _array_element) (`KismetStringLibrary.Conv_StringToName` (`|GetEnumeratorNameAsString` (`self.CurrentPhase`))))
      (`KismetArrayLibrary.Array_Add` (`self.CurrentAttacks`) _array_element)))
  (`self.StartAttack`)
  (set `self.IsActive` true))

(event `StartAttack`
  (bind _currentattackindex (`self.CurrentAttackIndex`))
  (bind _currentattacks (`self.CurrentAttacks`))
  (`KismetSystemLibrary.PrintString` (`KismetStringLibrary.Conv_IntToString` (`self.CurrentAttackIndex`)))
  (`/Game/Bosses/Attacks/BPC_BossAttack.StartAttack` (`|GetArrayItem` _currentattacks _currentattackindex))
  (`/Engine/EditorBlueprintResources/StandardMacros.IncrementInt` _currentattackindex
    (:`  `
      (if (== (`KismetArrayLibrary.Array_Length` _currentattacks) _currentattackindex)
        (set `self.CurrentAttackIndex` 0)))))

(event `NextPhase`
  (set `self.CurrentPhase` (cast `/Game/Bosses/Enum_Phases` (`KismetMathLibrary.Conv_IntToByte` (+ (`KismetMathLibrary.Conv_ByteToInt` (`self.CurrentPhase`)) 1))))
  (set `self.CurrentAttackIndex` 0)
  (`self.OnPhaseChange`)
  (`self.InitPhase`))

(event `ActivateBoss`
  (`/Engine/EditorBlueprintResources/StandardMacros.DoOnce` false
    (:`Completed`
      (`self.InitPhase`)
      (`self.CreateBossWidget`))))

(event `self.ReceiveAnyDamage`
  (params (Damage :type "Float (single-precision)") (DamageType :type "DamageType Object Reference") (InstigatedBy :type "Controller Object Reference") (DamageCauser :type "Actor Object Reference"))
  (bind _returnvalue (- (`self.HP`) Damage))
  (if (`self.IsActive`)
    (if (<= _returnvalue 0.0)
      (`self.PlayEndDialogue`)
      (`self.Drop`)
      (`self.K2_DestroyActor`)
      (else
        (set `self.HP` _returnvalue)))))

(event `PlayEndDialogue`
  (bind _returnvalue (`GameplayStatics.GetPlayerController` 0))
  (bind _returnvalue_2 (`GameplayStatics.GetPlayerCharacter` 0))
  (bind _returnvalue_3 (`|CreateWidget` (`self.EndDialogueWidget`)))
  (`UserWidget.AddToViewport` _returnvalue_3 0)
  (`WidgetBlueprintLibrary.SetInputMode_UIOnlyEx` _returnvalue null)
  (`self.DisableInput` _returnvalue_2 _returnvalue)
  (bind _asbp_character (cast `/Game/BaseBP/BP_Character` _returnvalue_2))
  (set `/Game/BaseBP/BP_Character.bIsFiring` false _asbp_character))

(event `Drop`
  (`|SpawnActorFromClass` (`self.DropItem`) (`KismetMathLibrary.MakeTransform` (`self.K2_GetActorLocation`)) "Undefined" "OverrideRootScale" null null))

(fn `UserConstructionScript`)