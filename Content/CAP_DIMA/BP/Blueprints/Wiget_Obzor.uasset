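; Trigger pickup actor that opens the Test_W widget when the player's BP_Character overlaps its Box.
; On overlap it plays a bonus sound, creates the widget, pauses the game, shows the widget on screen and destroys itself.
; BeginPlay caches the player character in BPAMMO, which is used only by disconnected ammo-refill logic that never runs.
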(event `self.ReceiveBeginPlay`
  ;[0 0 0] НАДО
  (bind _asbp_character (cast `/Game/BaseBP/BP_Character` (`GameplayStatics.GetPlayerCharacter` 0)))
  (set `self.BP_AMMO` _asbp_character))

(event `self.Box.OnComponentBeginOverlap`
  (params (OverlappedComponent :type "PrimitiveComponent Object Reference") (OtherActor :type "Actor Object Reference") (OtherComp :type "PrimitiveComponent Object Reference") (OtherBodyIndex :type Integer) (bFromSweep :type Boolean) (SweepResult :type "HitResult Structure (by ref)"))
  ;[0 0 0] Спавн
  (cast `/Game/BaseBP/BP_Character` OtherActor)
  (`GameplayStatics.PlaySound2D` "/Game/Alex/Sounds/SC_Bonus_Cue.SC_Bonus_Cue" 1.0 1.0 0.0 null null)
  (bind _returnvalue (`|CreateWidget` "/Game/Widget/Test_W.Test_W_C"))
  (`GameplayStatics.SetGamePaused` true)
  (`UserWidget.AddToViewport` _returnvalue 0)
  (`self.K2_DestroyActor`))

(fn `UserConstructionScript`)