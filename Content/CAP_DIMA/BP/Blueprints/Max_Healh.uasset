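; Health pickup actor that restores the player's health when walked into.
; On BeginPlay it caches player 0's character as a BP_Character reference.
; When that character overlaps the Box, it adds Healthamount to Health, clamped between 1 and MaxHealth, then destroys itself.
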(event `self.ReceiveBeginPlay`
  ;[0 0 0] НАДО
  (bind _asbp_character (cast `/Game/BaseBP/BP_Character` (`GameplayStatics.GetPlayerCharacter` 0)))
  (set `self.BP_Health` _asbp_character))

(event `self.Box.OnComponentBeginOverlap`
  (params (OverlappedComponent :type "PrimitiveComponent Object Reference") (OtherActor :type "Actor Object Reference") (OtherComp :type "PrimitiveComponent Object Reference") (OtherBodyIndex :type Integer) (bFromSweep :type Boolean) (SweepResult :type "HitResult Structure (by ref)"))
  (bind _bp_health (`self.BP_Health`))
  ;[0 0 0] Спавн
  (if (== OtherActor _bp_health)
    (set `/Game/BaseBP/BP_Character.Health` (`KismetMathLibrary.FClamp` (+ (`/Game/BaseBP/BP_Character.Health` _bp_health) (`self.Healthamount`)) 1.0 (`/Game/BaseBP/BP_Character.Max Health` _bp_health)) _bp_health)
    (`self.K2_DestroyActor`)))

(fn `UserConstructionScript`)