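; Max_Ammo is an ammo pickup actor that refills the player's ammo when touched.
; On BeginPlay it caches the player's BP_Character, and a Box overlap by that character adds a random large amount of ammo, clamped to a maximum.
; It then refreshes the ammo text on the player's HUD and destroys itself.
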(event `self.ReceiveBeginPlay`
  ;[0 0 0] НАДО
  (bind _asbp_character (cast `/Game/BaseBP/BP_Character` (`GameplayStatics.GetPlayerCharacter` 0)))
  (set `self.BP_AMMO` _asbp_character))

(event `self.Box.OnComponentBeginOverlap`
  (params (OverlappedComponent :type "PrimitiveComponent Object Reference") (OtherActor :type "Actor Object Reference") (OtherComp :type "PrimitiveComponent Object Reference") (OtherBodyIndex :type Integer) (bFromSweep :type Boolean) (SweepResult :type "HitResult Structure (by ref)"))
  (bind _bp_ammo (`self.BP_AMMO`))
  ;[0 0 0] Спавн
  (if (== OtherActor _bp_ammo)
    (set `/Game/BaseBP/BP_Character.Ammo` (`KismetMathLibrary.Clamp` (+ (`/Game/BaseBP/BP_Character.Ammo` _bp_ammo) (`KismetMathLibrary.RandomIntegerInRange` 90 120)) 0 150) _bp_ammo)
    (`/Game/Widget/PlayerHUD.UpdateAmmoText` (`/Game/BaseBP/BP_Character.PlayerHUD` _bp_ammo))
    (`self.K2_DestroyActor`)))

(fn `UserConstructionScript`)