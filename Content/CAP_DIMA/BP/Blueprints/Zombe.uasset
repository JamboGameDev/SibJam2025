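; Zombie enemy that roams, chases the player character and damages it on capsule contact.
; A looping AIMoveTo picks random navigable points but also passes the player as target actor, which overrides them.
; PawnSensing sightings start a chase, then a retriggerable delay clears the seen flag and resumes the roam loop.
; Damage spawns an emitter and reduces health; death ragdolls the mesh with an impulse and clears the sound timer.
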(event `Movearoundmap`
  ;[0 0 0] Навигатор-Не база
  (bind _randomlocation (`NavigationSystemV1.K2_GetRandomLocationInNavigableRadius` (`self.K2_GetActorLocation`) (`self.Radius`) null null :!label _label))
  (`|AIMoveTo` self _randomlocation (`self.BP`)
    (:`then`
      (`KismetSystemLibrary.Delay` (`self.Duration`))
      (if (not (`self.canseeplayer`))
        (goto _label)))))

(event `self.ReceiveBeginPlay`
  ;[0 0 0] Навигатор-Не база
  (bind _asbp_character (cast `/Game/CAP_DIMA/BP/Blueprints/BP_Character` (`GameplayStatics.GetPlayerCharacter` 0)))
  (set `self.BP` _asbp_character)
  (goto _label))

(event `self.PawnSensing.OnSeePawn`
  (params (Pawn :type "Pawn Object Reference"))
  ;[0 0 0] Ход
  (if (== Pawn (`self.BP`))
    (set `self.canseeplayer` true)
    (`|AIMoveTo` self (0.0 0.0 0.0) (`self.BP`)
      (:`then`
        (`KismetSystemLibrary.RetriggerableDelay` 3.0)
        (set `self.canseeplayer` false)
        (`self.Movearoundmap`)))))

(event `self.ReceiveAnyDamage`
  (params (Damage :type "Float (single-precision)") (DamageType :type "DamageType Object Reference") (InstigatedBy :type "Controller Object Reference") (DamageCauser :type "Actor Object Reference"))
  (bind _mesh (`self.Mesh`))
  (bind (_returnvalue_x _returnvalue_y) (`KismetMathLibrary.BreakVector` (* (`self.GetActorForwardVector` DamageCauser) 5000.0)))
  ;[0 0 0] Comment
  (`GameplayStatics.SpawnEmitterAttached` null (`self.Mesh`) "None" (`self.K2_GetActorLocation`) (struct) (1.0 1.0 1.0) "KeepWorldPosition")
  (bind _output_get (set `self.health` (- (`self.health`) Damage)))
  (if (<= _output_get 0.0)
    (`PrimitiveComponent.SetCollisionProfileName` _mesh "Ragdoll" true)
    (`PrimitiveComponent.SetSimulatePhysics` _mesh true)
    (`PrimitiveComponent.SetCollisionEnabled` (`self.CapsuleComponent`) "NoCollision")
    (`PrimitiveComponent.AddImpulse` _mesh (`KismetMathLibrary.MakeVector` _returnvalue_x _returnvalue_y) "None" true)
    (`KismetSystemLibrary.K2_ClearAndInvalidateTimerHandle` (`self.ZombeSound`))))

(event `self.CapsuleComponent.OnComponentHit`
  (params (HitComponent :type "PrimitiveComponent Object Reference") (OtherActor :type "Actor Object Reference") (OtherComp :type "PrimitiveComponent Object Reference") (NormalImpulse :type "Vector Structure") (Hit :type "HitResult Structure (by ref)"))
  (bind _bp (`self.BP`))
  ;[0 0 0] Удар-по игроку
  (if (== OtherActor _bp)
    (`GameplayStatics.ApplyDamage` _bp 1.0 null self)))

(event `self.ReceiveTick`
  (params (DeltaSeconds :type "Float (single-precision)"))
  ;[0 0 0] БАЗА
)

(event `CustomEvent`
  (params (Pawn :type "Pawn Object Reference"))
  ;[0 0 0] БАЗА
)

(fn `UserConstructionScript`)