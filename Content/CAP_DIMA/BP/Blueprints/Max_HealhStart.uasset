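; Health pickup that heals the player and shows the WB_Collect_Smetana screen when collected.
; Box overlap plays a sound and adds Healthamount to player 0's BP_Character Health, clamped between one and MaxHealth.
; The overlapping actor is checked only afterward, so any actor triggers the sound and heal.
; If it is a BP_Character, the widget appears, the game pauses and the pickup destroys itself.
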(event `self.Box.OnComponentBeginOverlap`
  (params (OverlappedComponent :type "PrimitiveComponent Object Reference") (OtherActor :type "Actor Object Reference") (OtherComp :type "PrimitiveComponent Object Reference") (OtherBodyIndex :type Integer) (bFromSweep :type Boolean) (SweepResult :type "HitResult Structure (by ref)"))
  ;[0 0 0] Спавн
  (`GameplayStatics.PlaySound2D` null 1.0 1.0 0.0 null null)
  (bind _asbp_character (cast `/Game/BaseBP/BP_Character` (`GameplayStatics.GetPlayerCharacter` 0)))
  (set `/Game/BaseBP/BP_Character.Health` (`KismetMathLibrary.FClamp` (+ (`/Game/BaseBP/BP_Character.Health` _asbp_character) (`self.Healthamount`)) 1.0 (`/Game/BaseBP/BP_Character.Max Health` _asbp_character)) _asbp_character)
  (cast `/Game/BaseBP/BP_Character` OtherActor)
  (bind _returnvalue (`|CreateWidget` "/Game/Alex/WB/WB_Collect_Smetana.WB_Collect_Smetana_C"))
  (`GameplayStatics.SetGamePaused` true)
  (`UserWidget.AddToViewport` _returnvalue 0)
  (`self.K2_DestroyActor`))

(fn `UserConstructionScript`)